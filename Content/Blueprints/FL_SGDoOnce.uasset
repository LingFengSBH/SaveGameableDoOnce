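; FL_SGDoOnce is a function library that exposes saving and restoring of DoOnce states held by the DoOnceSaverSubsystem.
; It gets or loads the whole state map, and clears it by loading an empty map.
; It also sets the state for a single object and removes invalid object keys, delegating all storage to the subsystem.
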(fn `ClearDoOnceState`
  (locals (EmptyMap :type "Map of Object Object Reference to DoOnceInfos Structure"))
  (`self.LoadDoOnceState` (`local.EmptyMap`)))

(fn `ClearInvalidDoOnceState`
  (`DoOnceSaverSubsystem.ClearInvalidObjectKeys` (subsystem `DoOnceSaverSubsystem`)))

(fn `GetDoOnceState`
  (returns (ReturnValue :type "Map of Object Object Reference to DoOnceInfos Structure"))
  (return (`DoOnceSaverSubsystem.GetHasDoneMap` (subsystem `DoOnceSaverSubsystem`))))

(fn `LoadDoOnceState`
  (params (DoOnceStateMap :type "Map of Object Object Reference to DoOnceInfos Structure (by ref)"))
  (`DoOnceSaverSubsystem.SetHasDoneMap` (subsystem `DoOnceSaverSubsystem`) DoOnceStateMap))

(fn `SetDoOnceStateToObject`
  (params (Object :type "Object Object Reference") (DoOnceState :type "DoOnceInfos Structure (by ref)"))
  (`DoOnceSaverSubsystem.SetHasDoneInfosOfObject` (subsystem `DoOnceSaverSubsystem`) Object (`.Info` (break `DoOnceInfos` DoOnceState))))